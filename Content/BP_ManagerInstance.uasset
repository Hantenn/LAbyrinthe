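; BP_ManagerInstance is a manager actor that spawns and clears instanced static meshes at runtime, grouped by mesh type.
; A map links each mesh to a HierarchicalInstancedStaticMesh component, created on demand when AjoutMesh first receives that mesh.
; AjoutMesh adds a world-space instance and returns its index, which EnleverInstanceMesh takes to remove it.
; Two other functions clear all instances of one mesh or of every mesh, keeping the components.
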(fn `AjoutMesh`
  (params (TypeMesh :type "StaticMesh Object Reference") (Transform :type "Transform Structure"))
  (returns (`Succes?` :type Boolean) (Index :type Integer))
  (bind (_value _returnvalue) (`BlueprintMapLibrary.Map_Find` (`self.InstanceComponent`) (`local.TypeMesh`)))
  (if _returnvalue
    (bind _returnvalue_2 (`InstancedStaticMeshComponent.AddInstance` _value (`local.Transform`) true))
    (return true _returnvalue_2)
    (else
      (bind _returnvalue_3 (`AddComponent|NODE_AddHierarchicalInstancedStaticMeshComponent-0`))
      (`BlueprintMapLibrary.Map_Add` (`self.InstanceComponent`) (`local.TypeMesh`) _returnvalue_3)
      (`StaticMeshComponent.SetStaticMesh` _returnvalue_3 (`local.TypeMesh`))
      (bind _returnvalue_4 (`InstancedStaticMeshComponent.AddInstance` _returnvalue_3 (`local.Transform`) true))
      (return true _returnvalue_4))))

(fn `EnleverInstanceMesh`
  (params (Mesh :type "StaticMesh Object Reference") (Index :type Integer))
  (returns (`Succes?` :type Boolean))
  (bind (_value _returnvalue) (`BlueprintMapLibrary.Map_Find` (`self.InstanceComponent`) (`local.Mesh`)))
  (if _returnvalue
    (bind _returnvalue_2 (`InstancedStaticMeshComponent.RemoveInstance` _value (`local.Index`)))
    (return _returnvalue_2)
    (else
      (return false))))

(fn `Enlevertouteslesinstance`
  (returns (`Succes?` :type Boolean))
  (bind _keys (`BlueprintMapLibrary.Map_Keys` (`self.InstanceComponent`)))
  (for _array_element _keys
    (`InstancedStaticMeshComponent.ClearInstances` (`BlueprintMapLibrary.Map_Find` (`self.InstanceComponent`) _array_element)))
  (return true))

(fn `Enlevertoutlesmesh`
  (params (Mesh :type "StaticMesh Object Reference"))
  (returns (`Succes?` :type Boolean))
  (bind (_value _returnvalue) (`BlueprintMapLibrary.Map_Find` (`self.InstanceComponent`) (`local.Mesh`)))
  (if _returnvalue
    (`InstancedStaticMeshComponent.ClearInstances` _value)
    (return true)
    (else
      (return false))))

(fn `UserConstructionScript`)